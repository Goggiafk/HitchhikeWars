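; BP_PlaceToSleep is a possessable sofa where the third-person player character can lie down and sleep.
; A box overlap shows an interact widget and arms the character's sleep-click event.
; Sleeping possesses this pawn, swaps to the sleep input context, moves the character to SleepPosition, and plays a looping single-node sleep animation.
; The exit input restores possession, default input and the animation Blueprint, then detaches and resets rotation.
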(event `self.ReceiveBeginPlay`
  (bind _output_get (set `self.PlayerCharacter` (`GameplayStatics.GetPlayerCharacter` 0)))
  (bind _asbp_third_person_character (cast `/Game/ThirdPerson/Blueprints/BP_ThirdPersonCharacter` _output_get))
  (add `/Game/ThirdPerson/Blueprints/BP_ThirdPersonCharacter.OnSleepEnterClick` _asbp_third_person_character (delegate `Sleep`)))

(event `Sleep`
  (if (`self.IsNearSofa`)
    (set `self.IsNearSofa` false)
    (`self.Enter Game`)))

(event `EnhancedInput|/Game/Inputs/IA_Exit`
  (params (ActionValue :type Boolean) (ElapsedSeconds :type "Float (double-precision)") (TriggeredSeconds :type "Float (double-precision)") (InputAction :type "InputAction Object Reference" :default "/Game/Inputs/IA_Exit.IA_Exit"))
  (bind _playercharacter (`self.PlayerCharacter`))
  (:`Started`
    (`EnhancedInputSubsystemInterface.RemoveMappingContext` (pcsubsystem `EnhancedInputLocalPlayerSubsystem` (`GameplayStatics.GetPlayerController` 0)) "/Game/Inputs/IMC_Sleep.IMC_Sleep" (make `ModifyContextOptions` true))
    (`Controller.Possess` (`GameplayStatics.GetPlayerController` 0) _playercharacter)
    (`SkeletalMeshComponent.SetAnimationMode` (`Character.Mesh` _playercharacter) "AnimationBlueprint")
    (`EnhancedInputSubsystemInterface.AddMappingContext` (pcsubsystem `EnhancedInputLocalPlayerSubsystem` (`GameplayStatics.GetPlayerController` 0)) "/Game/ThirdPerson/Input/IMC_Default.IMC_Default" 0 (make `ModifyContextOptions` true))
    (`self.K2_DetachFromActor` (`self.PlayerCharacter`) "KeepWorld" "KeepWorld" "KeepRelative")
    (`KismetSystemLibrary.Delay` 0.2)
    (`self.K2_SetActorRotation` :`self` (`self.PlayerCharacter`))))

(event `self.Box.OnComponentBeginOverlap`
  (params (OverlappedComponent :type "PrimitiveComponent Object Reference") (OtherActor :type "Actor Object Reference") (OtherComp :type "PrimitiveComponent Object Reference") (OtherBodyIndex :type Integer) (bFromSweep :type Boolean) (SweepResult :type "HitResult Structure (by ref)"))
  (bind _asbp_third_person_character (cast `/Game/ThirdPerson/Blueprints/BP_ThirdPersonCharacter` OtherActor))
  (if true
    (`/Engine/EditorBlueprintResources/StandardMacros.DoOnce` false :!label _label
      (:`Completed`
        (set `self.IsNearSofa` true)
        (bind _returnvalue (`|CreateWidget` "/Game/UI/CarTalks/WBP_InteractWithCar.WBP_InteractWithCar_C" (`self.GetLocalViewingPlayerController` _asbp_third_person_character)))
        (bind _output_get (set `self.InteractWidget` _returnvalue))
        (`UserWidget.AddToViewport` _output_get 0)))))

(event `self.Box.OnComponentEndOverlap`
  (params (OverlappedComponent :type "PrimitiveComponent Object Reference") (OtherActor :type "Actor Object Reference") (OtherComp :type "PrimitiveComponent Object Reference") (OtherBodyIndex :type Integer))
  (bind _interactwidget (`self.InteractWidget`))
  (bind _asbp_third_person_character (cast `/Game/ThirdPerson/Blueprints/BP_ThirdPersonCharacter` OtherActor))
  (if true
    (set `self.IsNearSofa` false)
    (`/Engine/EditorBlueprintResources/StandardMacros.IsValid` _interactwidget
      (:`Is Valid`
        (`Widget.RemoveFromParent` _interactwidget)
        (goto _label :!via `Reset`)))))

(event `Enter Game`
  (bind _sleepposition (`self.SleepPosition`))
  (bind _playercharacter (`self.PlayerCharacter`))
  (bind _interactwidget (`self.InteractWidget`))
  (bind _mesh (`Character.Mesh` _playercharacter))
  (`EnhancedInputSubsystemInterface.RemoveMappingContext` (pcsubsystem `EnhancedInputLocalPlayerSubsystem` (`GameplayStatics.GetPlayerController` 0)) "/Game/ThirdPerson/Input/IMC_Default.IMC_Default" (make `ModifyContextOptions` true))
  (`Controller.Possess` (`GameplayStatics.GetPlayerController` 0) self)
  (cast `/Game/ThirdPerson/Blueprints/BP_ThirdPersonCharacter` _playercharacter)
  (`self.K2_SetActorTransform` _playercharacter (`SceneComponent.K2_GetComponentToWorld` _sleepposition) false false)
  (`self.K2_SetActorRotation` _playercharacter (`SceneComponent.RelativeRotation` _sleepposition) false)
  (`SkeletalMeshComponent.SetAnimationMode` (`Character.Mesh` _playercharacter) "AnimationSingleNode")
  (`SkeletalMeshComponent.SetAnimation` _mesh "/Game/LowPolyMen/Animations/Animations/LPC_SleepingLaying_Sleeping_Anim_mixamo_com.LPC_SleepingLaying_Sleeping_Anim_mixamo_com")
  (`SkeletalMeshComponent.Play` _mesh true)
  (`EnhancedInputSubsystemInterface.AddMappingContext` (pcsubsystem `EnhancedInputLocalPlayerSubsystem` (`GameplayStatics.GetPlayerController` 0)) "/Game/Inputs/IMC_Sleep.IMC_Sleep" 0 (make `ModifyContextOptions` true))
  (`/Engine/EditorBlueprintResources/StandardMacros.IsValid` _interactwidget
    (:`Is Valid`
      (`Widget.RemoveFromParent` _interactwidget)
      (`self.K2_AttachToActor` (`self.PlayerCharacter`) self "None" "KeepWorld" "KeepWorld" "KeepWorld" true))))

(fn `UserConstructionScript`)