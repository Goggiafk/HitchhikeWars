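; Player controller that creates the game's main HUD widget on BeginPlay and switches between gameplay, menu, map and inventory screens.
; Enhanced Input actions change the active page of a widget switcher, pairing each change with the input mode and mouse cursor visibility.
; Menu toggles on each Started press, while map and inventory open on Started and return to the gameplay page only on Canceled.
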(event `self.ReceiveBeginPlay`
  (bind _returnvalue (`|CreateWidget` "/Game/UI/WBP_GameWidget.WBP_GameWidget_C"))
  (bind _output_get (set `self.GameWidget` _returnvalue))
  (`UserWidget.AddToViewport` _output_get 0))

(event `EnhancedInput|/Game/Inputs/IA_ToggleMap`
  (params (ActionValue :type Boolean) (ElapsedSeconds :type "Float (double-precision)") (TriggeredSeconds :type "Float (double-precision)") (InputAction :type "InputAction Object Reference" :default "/Game/Inputs/IA_ToggleMap.IA_ToggleMap"))
  (bind _returnvalue (`GameplayStatics.GetPlayerController` 0))
  (bind _widgetswitcher_37 (`/Game/UI/WBP_GameWidget.WidgetSwitcher_37` (`self.GameWidget`)))
  (:`Started`
    (`WidgetSwitcher.SetActiveWidgetIndex` _widgetswitcher_37 2)
    (`WidgetBlueprintLibrary.SetInputMode_UIOnlyEx` _returnvalue null)
    (set `PlayerController.bShowMouseCursor` true _returnvalue))
  (:`Canceled`
    (`WidgetSwitcher.SetActiveWidgetIndex` _widgetswitcher_37 0)
    (`WidgetBlueprintLibrary.SetInputMode_GameOnly` _returnvalue)
    (set `PlayerController.bShowMouseCursor` false _returnvalue)))

(event `EnhancedInput|/Game/Inputs/IA_ToggleMenu`
  (params (ActionValue :type Boolean) (ElapsedSeconds :type "Float (double-precision)") (TriggeredSeconds :type "Float (double-precision)") (InputAction :type "InputAction Object Reference" :default "/Game/Inputs/IA_ToggleMenu.IA_ToggleMenu"))
  (bind _returnvalue (`GameplayStatics.GetPlayerController` 0))
  (bind _widgetswitcher_37 (`/Game/UI/WBP_GameWidget.WidgetSwitcher_37` (`self.GameWidget`)))
  (:`Started`
    (if (== (`WidgetSwitcher.ActiveWidgetIndex` _widgetswitcher_37) 1)
      (`WidgetSwitcher.SetActiveWidgetIndex` _widgetswitcher_37 0)
      (`WidgetBlueprintLibrary.SetInputMode_GameOnly` _returnvalue)
      (set `PlayerController.bShowMouseCursor` false _returnvalue)
      (else
        (`WidgetSwitcher.SetActiveWidgetIndex` _widgetswitcher_37 1)
        (`WidgetBlueprintLibrary.SetInputMode_UIOnlyEx` _returnvalue null)
        (set `PlayerController.bShowMouseCursor` true _returnvalue)))))

(event `EnhancedInput|/Game/Inputs/IA_ToggleInventory`
  (params (ActionValue :type Boolean) (ElapsedSeconds :type "Float (double-precision)") (TriggeredSeconds :type "Float (double-precision)") (InputAction :type "InputAction Object Reference" :default "/Game/Inputs/IA_ToggleInventory.IA_ToggleInventory"))
  (bind _returnvalue (`GameplayStatics.GetPlayerController` 0))
  (bind _widgetswitcher_37 (`/Game/UI/WBP_GameWidget.WidgetSwitcher_37` (`self.GameWidget`)))
  (:`Started`
    (`WidgetSwitcher.SetActiveWidgetIndex` _widgetswitcher_37 3)
    (`WidgetBlueprintLibrary.SetInputMode_UIOnlyEx` _returnvalue null)
    (set `PlayerController.bShowMouseCursor` true _returnvalue))
  (:`Canceled`
    (`WidgetSwitcher.SetActiveWidgetIndex` _widgetswitcher_37 0)
    (`WidgetBlueprintLibrary.SetInputMode_GameOnly` _returnvalue)
    (set `PlayerController.bShowMouseCursor` false _returnvalue)))

(fn `UserConstructionScript`)